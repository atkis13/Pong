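; BP_Boundary is a Pong arena boundary actor that can act as a scoring goal.
; On BeginPlay it caches the PongGameMode.
; When a Ball overlaps a boundary flagged as a goal, it destroys the ball and increases the AI score for the left goal, or the player score otherwise.
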(event EventBeginPlay
  ;[1 1 1] Comment
  (bind _aspong_game_mode (Utilities|Casting|CastToPongGameMode (Game|GetGameMode)))
  (Variables|Default|SetGameModeRef _aspong_game_mode))

(event Collision|EventActorBeginOverlap
  (params (OtherActor :type Actor%20Object%20Reference))
  (bind _gamemoderef (Variables|Default|GetGameModeRef))
  ;[1 1 1] Comment
  (if (Variables|Default|GetIsGoal)
    (bind _asball (Utilities|Casting|CastToBall OtherActor))
    (Actor|DestroyActor _asball)
    (if (Variables|Default|GetIsLeftGoal)
      (Class|PongGameMode|IncreaseAIScore _gamemoderef)
      (else
        (Class|PongGameMode|IncreasePlayerScore _gamemoderef)))))

(fn ConstructionScript)